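; Display slot actor in the VR paint board system that holds a single painted canvas for display.
; It accepts a canvas only when empty and the canvas size is in its allowed list, which is filled on BeginPlay with two size enum values.
; Place and remove events set or clear the current canvas reference.
; Getters expose that canvas, a snap component for attachment, and an arrow-based view location.
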(event EventPlaceCanvas
  (params (Canvas :type Canvas%20Board%20BP%20Object%20Reference))
  (Variables|Claude|SetCurrent%20Canvas Canvas))

(event EventRemoveCanvas
  (Variables|Claude|SetCurrent%20Canvas 0))

(event EventBeginPlay
  (Variables|Claude|SetAccepted%20Sizes (Utilities|Array|MakeArray "NewEnumerator0" "NewEnumerator1")))

(fn ConstructionScript)

(fn CanAcceptCanvas?
  (params (Canvas :type Canvas%20Board%20BP%20Object%20Reference))
  (return (and (not (Utilities|IsValid (Variables|Claude|GetCurrent%20Canvas))) (Utilities|Array|ContainsItem (Variables|Claude|GetAccepted%20Sizes) (Variables|/Game/VR_PaintStuff/Paint_Board/Canvas_Board_BP.Canvas_Board_BP_C|GetCanvasSize Canvas)))))

(fn GetDisplayedCanvas
  (return (Variables|Claude|GetCurrent%20Canvas)))

(fn GetSnapComponent
  (return (Variables|Default|GetSnap%20Point)))

(fn GetViewLocation
  (return (Transformation|GetWorldLocation (Variables|Default|GetArrow1))))