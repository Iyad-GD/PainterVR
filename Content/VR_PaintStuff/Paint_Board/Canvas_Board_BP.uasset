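; Grabbable VR paint canvas board that can be painted with brushes and snapped onto display slots.
; On BeginPlay it creates a white render target shown through a dynamic board material, plus a dynamic brush material.
; DrawBrush stamps that material onto the target at a given location, size, color and texture.
; At startup or on drop it attaches to the first accepting overlapping Display_Slot_BP; grabbing releases the slot.
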(event OnGrabbed(BP_GrabComponent)
  ;[0 0.01958 0.15 0.5 60] Snap Logic
  (Utilities|IsValid (Variables|Claude|GetCurrentDisplay)
    (:Is%20Valid
      (Class|BPIDisplaySurface|RemoveCanvas(Message) (Variables|Claude|GetCurrentDisplay))
      (Variables|Claude|SetCurrentDisplay 0))))

(event OnDropped(BP_GrabComponent)
  ;[0 0.01958 0.15 0.5 60] Snap Logic
  (CallFunction|TryPlaceonDisplay))

(event EventBeginPlay
  (Utilities|FlowControl|Delay 0.2)
  (CallFunction|TryPlaceonDisplay)
  (Utilities|Array|Resize (Variables|PaintingStats|GetCoverage%20Grid) 256)
  ;[0.15 0.1401 0 0.5 60] Paint Logic
  (Utilities|FlowControl|Sequence
    (:then_0
      (bind _returnvalue (Rendering|CreateRenderTarget2D 1024 1024 "RTF_RGBA16f"))
      (bind _output_get (Variables|Drawing|SetRenderTarget _returnvalue))
      (Rendering|ClearRenderTarget2D _output_get "(R=1.000000,G=1.000000,B=1.000000,A=1.000000)")
      (Variables|Claude|SetCanvasSize "NewEnumerator0"))
    (:then_1
      (bind _returnvalue_2 (Rendering|Material|CreateDynamicMaterialInstance "/Game/VR_PaintStuff/Paint_Board/Materials_Textures/CanvasMat.CanvasMat" "None" "None" :!class /Script/Engine.KismetMaterialLibrary))
      (Rendering|Material|SetTextureParameterValue _returnvalue_2 "RenderTarget" (Variables|Drawing|GetRenderTarget))
      (Rendering|Material|SetMaterial (Variables|Default|GetBoard) 0 _returnvalue_2))
    (:then_2
      (bind _returnvalue_3 (Rendering|Material|CreateDynamicMaterialInstance "/Game/VR_PaintStuff/Paint_Board/Materials_Textures/Brush_Material.Brush_Material" "None" "None" :!class /Script/Engine.KismetMaterialLibrary))
      (Variables|Drawing|SetBrushMat _returnvalue_3))))

(fn ConstructionScript)

(fn DrawBrush
  (params (BrushTexture :type Texture%202D%20Object%20Reference) (BrushSize :type Float%20%28double-precision%29) (DrawLocation :type Vector%202D%20Structure) (Brush%20Color :type Linear%20Color%20Structure))
  (bind _brushmat (Variables|Drawing|GetBrushMat))
  (Utilities|FlowControl|Sequence
    (:then_0
      (Rendering|Material|SetTextureParameterValue _brushmat "TextureSample" BrushTexture)
      (Rendering|Material|SetVectorParameterValue _brushmat "Brush Color" Brush%20Color :!class /Script/Engine.MaterialInstanceDynamic))
    (:then_1
      (bind (_canvas _size _context) (Rendering|BeginDrawCanvastoRenderTarget (Variables|Drawing|GetRenderTarget)))
      (Canvas|DrawMaterial :self _canvas :RenderMaterial (Variables|Drawing|GetBrushMat) :ScreenPosition (- (* _size DrawLocation) (/ BrushSize 2.0)) :ScreenSize (Math|Vector2D|MakeVector2D BrushSize BrushSize) :CoordinateSize "(X=1.000000,Y=1.000000)" :PivotPoint "(X=0.500000,Y=0.500000)")
      (Rendering|EndDrawCanvastoRenderTarget _context))))

(fn SnaptoDisplay
  (params (Display :type Actor%20Object%20Reference))
  (Physics|SetSimulatePhysics (Variables|Default|GetBoard) false)
  (bind _snap_component (Class|BPIDisplaySurface|GetSnapComponent(Message) Display))
  (Transformation|AttachComponentToComponent self _snap_component "None" "SnapToTarget" "SnapToTarget" "KeepWorld" true)
  (bind _output_get (Variables|Claude|SetCurrentDisplay Display))
  (Class|BPIDisplaySurface|PlaceCanvas(Message) Display self)
  (Development|PrintString (Utilities|GetDisplayName _output_get)))

(fn TryPlaceonDisplay
  (bind _array_element (Utilities|Array|ForEachLoopwithBreak (Collision|GetOverlappingActors (Variables|Default|GetBoard) "/Game/VR_PaintStuff/Paint_Board/DisplaySlot/Display_Slot_BP.Display_Slot_BP_C" :!class /Script/Engine.PrimitiveComponent) :!label _label)
    (:LoopBody
      (bind _can_accept_ (Class|BPIDisplaySurface|CanAcceptCanvas?(Message) _array_element self))
      (if _can_accept_
        (CallFunction|SnaptoDisplay _array_element)
        (goto _label Break)))))